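; Main-menu load Blueprint for the FreightDock mod that registers options with the mod API.
; On BeginPlay it binds a handler to the API's option-changed event, then calls RegisterOptions after a short delay.
; OptionChanged calls RegisterOptions again when the language setting changes.
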(event `self.ReceiveBeginPlay`
  (add `ModAPI.onOptionChanged` (`ModAPI.GetModAPI`) (`|CreateDelegate` :!event `OptionChanged`))
  (`KismetSystemLibrary.Delay` 0.2)
  (`/Game/Mods/FreightDock/Loom/BPL_FDOptions.RegisterOptions` (`ModAPI.GetModAPI`)))

(fn `OptionChanged`
  (params (optionId :type String) (Value :type String))
  (if (`KismetStringLibrary.EqualEqual_StrStr` optionId "settings.language")
    (`/Game/Mods/FreightDock/Loom/BPL_FDOptions.RegisterOptions` (`ModAPI.GetModAPI`))))