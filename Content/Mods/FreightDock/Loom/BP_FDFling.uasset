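; One-shot effect actor that flings haul meshes in arcs from itself to a partner's owner, showing goods gained in the partner's sea-goods stockpile.
; Before snapshots slot counts; Launch diffs them and converts gains into a capped piece count, trimming the largest shares and interleaving resource types.
; Tick moves pooled, collision-free mesh components along staggered, spinning parabolas scaled by distance, then destroys the actor when all land.
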(event `self.ReceiveBeginPlay`
  (`self.Loom_On_ReceiveBeginPlay`))

(event `self.ReceiveTick`
  (params (DeltaSeconds :type "Float (single-precision)"))
  (`self.Loom_On_ReceiveTick` DeltaSeconds))

(fn `Before`
  (params (Partner :type "WorkDock Object Reference"))
  (locals (Loom_Index4 :type Integer))
  (bind _slots (break `Stockpile` (`WorkDock.m_stockpile_goodsFromSea` Partner)))
  (bind _keys (`BlueprintMapLibrary.Map_Keys` _slots))
  (set `local.Loom_Index4` 0)
  (if (< (`local.Loom_Index4`) (`KismetArrayLibrary.Array_Length` _keys)) :!label _label
    (bind _output (`|GetArrayItem` _keys (`local.Loom_Index4`)))
    (`BlueprintMapLibrary.Map_Add` (`self.Had`) _output (`.count` (break `ResourceStockpileSlot` (`BlueprintMapLibrary.Map_Find` _slots _output))))
    (set `local.Loom_Index4` (+ (`local.Loom_Index4`) 1))
    (goto _label)))

(fn `Duration`
  (returns (ReturnValue :type "Float (double-precision)"))
  (return 0.8))

(fn `Launch`
  (params (Partner :type "WorkDock Object Reference"))
  (locals (names :type "Array of Name") (amounts :type "Array of Integer") (Loom_Index8 :type Integer) (Loom_If21 :type Integer) (gained :type Integer) (counts :type "Array of Integer") (total :type Integer) (i :type Integer) (n :type Integer) (big :type Integer) (round :type Integer) (def :type "ResourceDef Structure") (dx :type "Float (double-precision)") (dy :type "Float (double-precision)"))
  (bind _slots (break `Stockpile` (`WorkDock.m_stockpile_goodsFromSea` Partner)))
  (`KismetArrayLibrary.Array_Clear` (`local.names`))
  (`KismetArrayLibrary.Array_Clear` (`local.amounts`))
  (bind _keys (`BlueprintMapLibrary.Map_Keys` _slots))
  (set `local.Loom_Index8` 0)
  (if (< (`local.Loom_Index8`) (`KismetArrayLibrary.Array_Length` _keys)) :!label _label
    (bind _output (`|GetArrayItem` _keys (`local.Loom_Index8`)))
    (bind (_value _returnvalue) (`BlueprintMapLibrary.Map_Find` (`self.Had`) _output))
    (if _returnvalue
      (set `local.Loom_If21` _value)
      (else
        (set `local.Loom_If21` 0)))
    (set `local.gained` (- (`.count` (break `ResourceStockpileSlot` (`BlueprintMapLibrary.Map_Find` _slots _output))) (`local.Loom_If21`)))
    (if (> (`local.gained`) 0)
      (`KismetArrayLibrary.Array_Add` (`local.names`) _output)
      (`KismetArrayLibrary.Array_Add` (`local.amounts`) (`local.gained`)))
    (set `local.Loom_Index8` (+ (`local.Loom_Index8`) 1))
    (goto _label)
    (else
      (`KismetArrayLibrary.Array_Clear` (`local.counts`))
      (set `local.total` 0)
      (set `local.i` 0)
      (if (< (`local.i`) (`KismetArrayLibrary.Array_Length` (`local.names`))) :!label _label_2
        (set `local.n` (`KismetMathLibrary.Max` (/ (`|GetArrayItem` (`local.amounts`) (`local.i`)) (`self.PerPiece`)) 1))
        (`KismetArrayLibrary.Array_Add` (`local.counts`) (`local.n`))
        (set `local.total` (+ (`local.total`) (`local.n`)))
        (set `local.i` (+ (`local.i`) 1))
        (goto _label_2)
        (else
          (if (> (`local.total`) (`self.MaxPieces`)) :!label _label_3
            (set `local.big` (- 0 1))
            (set `local.i` 0)
            (if (< (`local.i`) (`KismetArrayLibrary.Array_Length` (`local.counts`))) :!label _label_4
              (if (> (`|GetArrayItem` (`local.counts`) (`local.i`)) 1)
                (if (or (< (`local.big`) 0) (> (`|GetArrayItem` (`local.counts`) (`local.i`)) (`|GetArrayItem` (`local.counts`) (`local.big`))))
                  (set `local.big` (`local.i`))))
              (set `local.i` (+ (`local.i`) 1))
              (goto _label_4)
              (elif (< (`local.big`) 0)
                (set `local.total` (`self.MaxPieces`))
                (goto _label_3)
                (else
                  (`KismetArrayLibrary.Array_Set` (`local.counts`) (`local.big`) (- (`|GetArrayItem` (`local.counts`) (`local.big`)) 1))
                  (set `local.total` (- (`local.total`) 1))
                  (goto _label_3))))
            (else
              (set `self.Used` 0)
              (`KismetArrayLibrary.Array_Clear` (`self.Starts`))
              (set `local.round` 0)
              (if (and (< (`self.Used`) (`self.MaxPieces`)) (< (`local.round`) (`self.MaxPieces`))) :!label _label_5
                (set `local.i` 0)
                (if (< (`local.i`) (`KismetArrayLibrary.Array_Length` (`local.names`))) :!label _label_6
                  (if (and (> (`|GetArrayItem` (`local.counts`) (`local.i`)) (`local.round`)) (< (`self.Used`) (`self.MaxPieces`)))
                    (bind _returnvalue_2 (`ArcoGameInstance.GetResourceDefCopy` self (`|GetArrayItem` (`local.names`) (`local.i`))))
                    (set `local.def` _returnvalue_2)
                    (`StaticMeshComponent.SetStaticMesh` (`|GetArrayItem` (`self.Pieces`) (`self.Used`)) (`.haulMesh` (break `ResourceDef` (`local.def`))))
                    (`KismetArrayLibrary.Array_Add` (`self.Starts`) (* (`KismetMathLibrary.Conv_IntToDouble` (`self.Used`)) (`self.Stagger`)))
                    (set `self.Used` (+ (`self.Used`) 1)))
                  (set `local.i` (+ (`local.i`) 1))
                  (goto _label_6)
                  (else
                    (set `local.round` (+ (`local.round`) 1))
                    (goto _label_5)))
                (elif (== (`self.Used`) 0)
                  (`self.K2_DestroyActor`)
                  (return)
                  (else
                    (set `self.From` (`self.K2_GetActorLocation`))
                    (set `self.To` (`self.K2_GetActorLocation` (`ActorComponent.GetOwner` Partner)))
                    (set `local.dx` (- (.x (`self.To`)) (.x (`self.From`))))
                    (set `local.dy` (- (.y (`self.To`)) (.y (`self.From`))))
                    (set `self.Height` (`KismetMathLibrary.FClamp` (* (`KismetMathLibrary.Sqrt` (+ (* (`local.dx`) (`local.dx`)) (* (`local.dy`) (`local.dy`)))) 0.35) 150.0 1000.0))
                    (set `self.Began` (`GameplayStatics.GetTimeSeconds`))))))))))))

(fn `Loom_On_ReceiveBeginPlay`
  (locals (Loom_Index112 :type Integer))
  (bind _pieces (`self.Pieces`))
  (bind _output (`|GetArrayItem` _pieces (`local.Loom_Index112`)))
  (`KismetArrayLibrary.Array_Clear` (`self.Pieces`))
  (`KismetArrayLibrary.Array_Add` (`self.Pieces`) (`self.P0`))
  (`KismetArrayLibrary.Array_Add` (`self.Pieces`) (`self.P1`))
  (`KismetArrayLibrary.Array_Add` (`self.Pieces`) (`self.P2`))
  (`KismetArrayLibrary.Array_Add` (`self.Pieces`) (`self.P3`))
  (`KismetArrayLibrary.Array_Add` (`self.Pieces`) (`self.P4`))
  (`KismetArrayLibrary.Array_Add` (`self.Pieces`) (`self.P5`))
  (`KismetArrayLibrary.Array_Add` (`self.Pieces`) (`self.P6`))
  (`KismetArrayLibrary.Array_Add` (`self.Pieces`) (`self.P7`))
  (`KismetArrayLibrary.Array_Add` (`self.Pieces`) (`self.P8`))
  (`KismetArrayLibrary.Array_Add` (`self.Pieces`) (`self.P9`))
  (`KismetArrayLibrary.Array_Add` (`self.Pieces`) (`self.P10`))
  (`KismetArrayLibrary.Array_Add` (`self.Pieces`) (`self.P11`))
  (`KismetArrayLibrary.Array_Add` (`self.Pieces`) (`self.P12`))
  (`KismetArrayLibrary.Array_Add` (`self.Pieces`) (`self.P13`))
  (`KismetArrayLibrary.Array_Add` (`self.Pieces`) (`self.P14`))
  (`KismetArrayLibrary.Array_Add` (`self.Pieces`) (`self.P15`))
  (`KismetArrayLibrary.Array_Add` (`self.Pieces`) (`self.P16`))
  (`KismetArrayLibrary.Array_Add` (`self.Pieces`) (`self.P17`))
  (`KismetArrayLibrary.Array_Add` (`self.Pieces`) (`self.P18`))
  (`KismetArrayLibrary.Array_Add` (`self.Pieces`) (`self.P19`))
  (`KismetArrayLibrary.Array_Add` (`self.Pieces`) (`self.P20`))
  (`KismetArrayLibrary.Array_Add` (`self.Pieces`) (`self.P21`))
  (`KismetArrayLibrary.Array_Add` (`self.Pieces`) (`self.P22`))
  (`KismetArrayLibrary.Array_Add` (`self.Pieces`) (`self.P23`))
  (`KismetArrayLibrary.Array_Add` (`self.Pieces`) (`self.P24`))
  (`KismetArrayLibrary.Array_Add` (`self.Pieces`) (`self.P25`))
  (`KismetArrayLibrary.Array_Add` (`self.Pieces`) (`self.P26`))
  (`KismetArrayLibrary.Array_Add` (`self.Pieces`) (`self.P27`))
  (`KismetArrayLibrary.Array_Add` (`self.Pieces`) (`self.P28`))
  (`KismetArrayLibrary.Array_Add` (`self.Pieces`) (`self.P29`))
  (`KismetArrayLibrary.Array_Add` (`self.Pieces`) (`self.P30`))
  (`KismetArrayLibrary.Array_Add` (`self.Pieces`) (`self.P31`))
  (`KismetArrayLibrary.Array_Add` (`self.Pieces`) (`self.P32`))
  (`KismetArrayLibrary.Array_Add` (`self.Pieces`) (`self.P33`))
  (`KismetArrayLibrary.Array_Add` (`self.Pieces`) (`self.P34`))
  (`KismetArrayLibrary.Array_Add` (`self.Pieces`) (`self.P35`))
  (set `local.Loom_Index112` 0)
  (if (< (`local.Loom_Index112`) (`KismetArrayLibrary.Array_Length` _pieces)) :!label _label
    (`PrimitiveComponent.SetCollisionEnabled` _output "NoCollision")
    (`SceneComponent.SetVisibility` _output false false)
    (set `local.Loom_Index112` (+ (`local.Loom_Index112`) 1))
    (goto _label)))

(fn `Loom_On_ReceiveTick`
  (params (dt :type "Float (double-precision)"))
  (locals (since :type "Float (double-precision)") (flying :type Boolean) (i :type Integer) (p :type "StaticMeshComponent Object Reference") (t :type "Float (double-precision)") (lift :type "Float (double-precision)") (at :type "Vector Structure"))
  (if (< (`self.Began`) 0.0)
    (return)
    (else
      (set `local.since` (- (`GameplayStatics.GetTimeSeconds`) (`self.Began`)))
      (set `local.flying` false)
      (set `local.i` 0)
      (if (< (`local.i`) (`self.Used`)) :!label _label
        (set `local.p` (`|GetArrayItem` (`self.Pieces`) (`local.i`)))
        (set `local.t` (/ (- (`local.since`) (`|GetArrayItem` (`self.Starts`) (`local.i`))) (`self.Duration`)))
        (if (< (`local.t`) 0.0)
          (set `local.flying` true)
          (elif (< (`local.t`) 1.0)
            (set `local.flying` true)
            (set `local.lift` (* (* (* 4.0 (`self.Height`)) (`local.t`)) (- 1.0 (`local.t`))))
            (set `local.at` (`KismetMathLibrary.MakeVector` (+ (.x (`self.From`)) (* (- (.x (`self.To`)) (.x (`self.From`))) (`local.t`))) (+ (.y (`self.From`)) (* (- (.y (`self.To`)) (.y (`self.From`))) (`local.t`))) (+ (+ (.z (`self.From`)) (* (- (.z (`self.To`)) (.z (`self.From`))) (`local.t`))) (`local.lift`))))
            (`SceneComponent.K2_SetWorldLocationAndRotation` (`local.p`) (`local.at`) (`KismetMathLibrary.MakeRotator` 0.0 (* (`local.t`) 360.0) (* (`KismetMathLibrary.Conv_IntToDouble` (`local.i`)) 40.0)) false false)
            (`SceneComponent.SetVisibility` (`local.p`) true false)
            (else
              (`SceneComponent.SetVisibility` (`local.p`) false false))))
        (set `local.i` (+ (`local.i`) 1))
        (goto _label)
        (elif (not (`local.flying`))
          (`self.K2_DestroyActor`))))))

(fn `MaxPieces`
  (returns (ReturnValue :type Integer))
  (return 36))

(fn `PerPiece`
  (returns (ReturnValue :type Integer))
  (return 4))

(fn `Stagger`
  (returns (ReturnValue :type "Float (double-precision)"))
  (return 0.07))