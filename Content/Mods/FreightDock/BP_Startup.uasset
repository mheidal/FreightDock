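; Startup actor for the Freight Dock mod that registers the mod's content through the ModAPI on BeginPlay.
; It adds a freightDock building row by copying navaltradeDock fields, then overrides the actor class, name, description and toolbar sort.
; It registers options for the dock pairing key and partial-load departure wait.
; It also adds a Stevedore carry-capacity modifier based on constructionyardWorker, with strings and log messages.
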(event `self.ReceiveBeginPlay`
  (set `self.ModAPI` (`ModAPI.GetModAPI`))
  (`self.RegisterFreightDock`)
  (`self.RegisterOptions`)
  (`self.RegisterExtras`))

(fn `RegisterExtras`
  (bind _map (`|MakeMap` "mod.stevedore" "Stevedore" "mod.desc.stevedore" "+10 carry capacity while working at a freight dock" :!type "Name"))
  (bind _modapi (`self.ModAPI`))
  (bind _returnvalue (`ModAPI.AddDataTableRow` _modapi "AgentModifiers" "mod.stevedore" :!pinned true)) ; AddMod
  (bind _returnvalue_2 (`ModAPI.ReadDataTableValue` _modapi "AgentModifiers" "mod.constructionyardWorker" "Icon" :!pinned true)) ; ModGet_Icon
  (`ModAPI.WriteDataTableValue` _modapi "AgentModifiers" "mod.stevedore" "Icon" _returnvalue_2 :!pinned true) ; ModSet_Icon
  (bind _returnvalue_3 (`ModAPI.ReadDataTableValue` _modapi "AgentModifiers" "mod.constructionyardWorker" "Category" :!pinned true)) ; ModGet_Category
  (`ModAPI.WriteDataTableValue` _modapi "AgentModifiers" "mod.stevedore" "Category" _returnvalue_3 :!pinned true) ; ModSet_Category
  (bind _returnvalue_4 (`ModAPI.ReadDataTableValue` _modapi "AgentModifiers" "mod.constructionyardWorker" "severity_mastersync" :!pinned true)) ; ModGet_severity_mastersync
  (`ModAPI.WriteDataTableValue` _modapi "AgentModifiers" "mod.stevedore" "severity_mastersync" _returnvalue_4 :!pinned true) ; ModSet_severity_mastersync
  (bind _returnvalue_5 (`ModAPI.ReadDataTableValue` _modapi "AgentModifiers" "mod.constructionyardWorker" "useResourceData" :!pinned true)) ; ModGet_useResourceData
  (`ModAPI.WriteDataTableValue` _modapi "AgentModifiers" "mod.stevedore" "useResourceData" _returnvalue_5 :!pinned true) ; ModSet_useResourceData
  (`ModAPI.WriteDataTableValue` _modapi "AgentModifiers" "mod.stevedore" "DisplayName" "mod.stevedore" :!pinned true) ; ModSet_DisplayName
  (`ModAPI.WriteDataTableValue` _modapi "AgentModifiers" "mod.stevedore" "Description" "mod.desc.stevedore" :!pinned true) ; ModSet_Description
  (`ModAPI.WriteDataTableValue` _modapi "AgentModifiers" "mod.stevedore" "carryMod" "10" :!pinned true) ; ModSet_carryMod
  (`ModAPI.WriteDataTableValue` _modapi "AgentModifiers" "mod.stevedore" "productivityMod" "0" :!pinned true) ; ModSet_productivityMod
  (`ModAPI.WriteDataTableValue` _modapi "AgentModifiers" "mod.stevedore" "speedMod" "0" :!pinned true) ; ModSet_speedMod
  (`ModAPI.WriteDataTableValue` _modapi "AgentModifiers" "mod.stevedore" "additionalStacks" "0" :!pinned true) ; ModSet_additionalStacks
  (`ModAPI.WriteDataTableValue` _modapi "AgentModifiers" "mod.stevedore" "canStack" "False" :!pinned true) ; ModSet_canStack
  (`ModAPI.WriteDataTableValue` _modapi "AgentModifiers" "mod.stevedore" "expires" "False" :!pinned true) ; ModSet_expires
  (`ModAPI.WriteDataTableValue` _modapi "AgentModifiers" "mod.stevedore" "hiddenMod" "False" :!pinned true) ; ModSet_hiddenMod
  (`ModAPI.AddNewStrings` _modapi "dev" _map :!pinned true) ; Strings_dev
  (`ModAPI.AddNewStrings` _modapi "en" _map :!pinned true) ; Strings_en
  (`ModAPI.LogMessage` _modapi (`KismetStringLibrary.Concat_StrStr` (`KismetStringLibrary.Concat_StrStr` "" "Stevedore modifier added: ") (`KismetStringLibrary.Conv_BoolToString` _returnvalue)) true :!pinned true) ; LogDone
)

(fn `RegisterFreightDock`
  (bind _map (`|MakeMap` "freightdock.building.freightDock" "Freight Dock" "freightdock.building.freightDock.desc" "Crew a ship that carries goods your paired freight dock's island needs, then returns" :!type "Name"))
  (bind _modapi (`self.ModAPI`))
  (bind _returnvalue (`ModAPI.ReadDataTableValue` _modapi "GridActors" "navaltradeDock" "GridActor"))
  (bind _returnvalue_2 (`ModAPI.AddDataTableRow` _modapi "GridActors" "freightDock"))
  (`ModAPI.WriteDataTableValue` _modapi "GridActors" "freightDock" "Description" "freightdock.building.freightDock.desc")
  (`ModAPI.WriteDataTableValue` _modapi "GridActors" "freightDock" "GridActor" "/Script/Engine.BlueprintGeneratedClass'/Game/Mods/FreightDock/navaldock_freight.navaldock_freight_C'")
  (bind _returnvalue_3 (`ModAPI.ReadDataTableValue` _modapi "GridActors" "navaltradeDock" "Icon"))
  (`ModAPI.WriteDataTableValue` _modapi "GridActors" "freightDock" "Icon" _returnvalue_3)
  (bind _returnvalue_4 (`ModAPI.ReadDataTableValue` _modapi "GridActors" "navaltradeDock" "Quality"))
  (`ModAPI.WriteDataTableValue` _modapi "GridActors" "freightDock" "Quality" _returnvalue_4)
  (bind _returnvalue_5 (`ModAPI.ReadDataTableValue` _modapi "GridActors" "navaltradeDock" "SupportedImprovements"))
  (`ModAPI.WriteDataTableValue` _modapi "GridActors" "freightDock" "SupportedImprovements" _returnvalue_5)
  (bind _returnvalue_6 (`ModAPI.ReadDataTableValue` _modapi "GridActors" "navaltradeDock" "TooltipTags"))
  (`ModAPI.WriteDataTableValue` _modapi "GridActors" "freightDock" "TooltipTags" _returnvalue_6)
  (bind _returnvalue_7 (`ModAPI.ReadDataTableValue` _modapi "GridActors" "navaltradeDock" "Variants"))
  (`ModAPI.WriteDataTableValue` _modapi "GridActors" "freightDock" "Variants" _returnvalue_7)
  (bind _returnvalue_8 (`ModAPI.ReadDataTableValue` _modapi "GridActors" "navaltradeDock" "asHouseTier"))
  (`ModAPI.WriteDataTableValue` _modapi "GridActors" "freightDock" "asHouseTier" _returnvalue_8)
  (bind _returnvalue_9 (`ModAPI.ReadDataTableValue` _modapi "GridActors" "navaltradeDock" "asIndustryDef"))
  (`ModAPI.WriteDataTableValue` _modapi "GridActors" "freightDock" "asIndustryDef" _returnvalue_9)
  (bind _returnvalue_10 (`ModAPI.ReadDataTableValue` _modapi "GridActors" "navaltradeDock" "catalyst"))
  (`ModAPI.WriteDataTableValue` _modapi "GridActors" "freightDock" "catalyst" _returnvalue_10)
  (bind _returnvalue_11 (`ModAPI.ReadDataTableValue` _modapi "GridActors" "navaltradeDock" "constructionTime"))
  (`ModAPI.WriteDataTableValue` _modapi "GridActors" "freightDock" "constructionTime" _returnvalue_11)
  (bind _returnvalue_12 (`ModAPI.ReadDataTableValue` _modapi "GridActors" "navaltradeDock" "cost1"))
  (`ModAPI.WriteDataTableValue` _modapi "GridActors" "freightDock" "cost1" _returnvalue_12)
  (bind _returnvalue_13 (`ModAPI.ReadDataTableValue` _modapi "GridActors" "navaltradeDock" "cost2"))
  (`ModAPI.WriteDataTableValue` _modapi "GridActors" "freightDock" "cost2" _returnvalue_13)
  (bind _returnvalue_14 (`ModAPI.ReadDataTableValue` _modapi "GridActors" "navaltradeDock" "cost3"))
  (`ModAPI.WriteDataTableValue` _modapi "GridActors" "freightDock" "cost3" _returnvalue_14)
  (bind _returnvalue_15 (`ModAPI.ReadDataTableValue` _modapi "GridActors" "navaltradeDock" "cost4"))
  (`ModAPI.WriteDataTableValue` _modapi "GridActors" "freightDock" "cost4" _returnvalue_15)
  (bind _returnvalue_16 (`ModAPI.ReadDataTableValue` _modapi "GridActors" "navaltradeDock" "ct1"))
  (`ModAPI.WriteDataTableValue` _modapi "GridActors" "freightDock" "ct1" _returnvalue_16)
  (bind _returnvalue_17 (`ModAPI.ReadDataTableValue` _modapi "GridActors" "navaltradeDock" "ct2"))
  (`ModAPI.WriteDataTableValue` _modapi "GridActors" "freightDock" "ct2" _returnvalue_17)
  (bind _returnvalue_18 (`ModAPI.ReadDataTableValue` _modapi "GridActors" "navaltradeDock" "ct3"))
  (`ModAPI.WriteDataTableValue` _modapi "GridActors" "freightDock" "ct3" _returnvalue_18)
  (bind _returnvalue_19 (`ModAPI.ReadDataTableValue` _modapi "GridActors" "navaltradeDock" "ct4"))
  (`ModAPI.WriteDataTableValue` _modapi "GridActors" "freightDock" "ct4" _returnvalue_19)
  (bind _returnvalue_20 (`ModAPI.ReadDataTableValue` _modapi "GridActors" "navaltradeDock" "customBuildCue"))
  (`ModAPI.WriteDataTableValue` _modapi "GridActors" "freightDock" "customBuildCue" _returnvalue_20)
  (bind _returnvalue_21 (`ModAPI.ReadDataTableValue` _modapi "GridActors" "navaltradeDock" "decorType"))
  (`ModAPI.WriteDataTableValue` _modapi "GridActors" "freightDock" "decorType" _returnvalue_21)
  (bind _returnvalue_22 (`ModAPI.ReadDataTableValue` _modapi "GridActors" "navaltradeDock" "detailCue"))
  (`ModAPI.WriteDataTableValue` _modapi "GridActors" "freightDock" "detailCue" _returnvalue_22)
  (bind _returnvalue_23 (`ModAPI.ReadDataTableValue` _modapi "GridActors" "navaltradeDock" "guildSpecialty"))
  (`ModAPI.WriteDataTableValue` _modapi "GridActors" "freightDock" "guildSpecialty" _returnvalue_23)
  (bind _returnvalue_24 (`ModAPI.ReadDataTableValue` _modapi "GridActors" "navaltradeDock" "hardLabor"))
  (`ModAPI.WriteDataTableValue` _modapi "GridActors" "freightDock" "hardLabor" _returnvalue_24)
  (bind _returnvalue_25 (`ModAPI.ReadDataTableValue` _modapi "GridActors" "navaltradeDock" "industrialLabor"))
  (`ModAPI.WriteDataTableValue` _modapi "GridActors" "freightDock" "industrialLabor" _returnvalue_25)
  (bind _returnvalue_26 (`ModAPI.ReadDataTableValue` _modapi "GridActors" "navaltradeDock" "isDraggableWall"))
  (`ModAPI.WriteDataTableValue` _modapi "GridActors" "freightDock" "isDraggableWall" _returnvalue_26)
  (bind _returnvalue_27 (`ModAPI.ReadDataTableValue` _modapi "GridActors" "navaltradeDock" "limitOne"))
  (`ModAPI.WriteDataTableValue` _modapi "GridActors" "freightDock" "limitOne" _returnvalue_27)
  (bind _returnvalue_28 (`ModAPI.ReadDataTableValue` _modapi "GridActors" "navaltradeDock" "maxAgents_contextual"))
  (`ModAPI.WriteDataTableValue` _modapi "GridActors" "freightDock" "maxAgents_contextual" _returnvalue_28)
  (bind _returnvalue_29 (`ModAPI.ReadDataTableValue` _modapi "GridActors" "navaltradeDock" "maxHealth"))
  (`ModAPI.WriteDataTableValue` _modapi "GridActors" "freightDock" "maxHealth" _returnvalue_29)
  (bind _returnvalue_30 (`ModAPI.ReadDataTableValue` _modapi "GridActors" "navaltradeDock" "minMaintenanceInterval"))
  (`ModAPI.WriteDataTableValue` _modapi "GridActors" "freightDock" "minMaintenanceInterval" _returnvalue_30)
  (bind _returnvalue_31 (`ModAPI.ReadDataTableValue` _modapi "GridActors" "navaltradeDock" "norefund"))
  (`ModAPI.WriteDataTableValue` _modapi "GridActors" "freightDock" "norefund" _returnvalue_31)
  (bind _returnvalue_32 (`ModAPI.ReadDataTableValue` _modapi "GridActors" "navaltradeDock" "randomlyRotate"))
  (`ModAPI.WriteDataTableValue` _modapi "GridActors" "freightDock" "randomlyRotate" _returnvalue_32)
  (bind _returnvalue_33 (`ModAPI.ReadDataTableValue` _modapi "GridActors" "navaltradeDock" "refundRule"))
  (`ModAPI.WriteDataTableValue` _modapi "GridActors" "freightDock" "refundRule" _returnvalue_33)
  (bind _returnvalue_34 (`ModAPI.ReadDataTableValue` _modapi "GridActors" "navaltradeDock" "requiresConstruction"))
  (`ModAPI.WriteDataTableValue` _modapi "GridActors" "freightDock" "requiresConstruction" _returnvalue_34)
  (`ModAPI.WriteDataTableValue` _modapi "GridActors" "freightDock" "stringKey" "freightdock.building.freightDock")
  (bind _returnvalue_35 (`ModAPI.ReadDataTableValue` _modapi "GridActors" "navaltradeDock" "structureType"))
  (`ModAPI.WriteDataTableValue` _modapi "GridActors" "freightDock" "structureType" _returnvalue_35)
  (bind _returnvalue_36 (`ModAPI.ReadDataTableValue` _modapi "GridActors" "navaltradeDock" "supportedIndustryRecipes"))
  (`ModAPI.WriteDataTableValue` _modapi "GridActors" "freightDock" "supportedIndustryRecipes" _returnvalue_36)
  (bind _returnvalue_37 (`ModAPI.ReadDataTableValue` _modapi "GridActors" "navaltradeDock" "toolbarGroup"))
  (`ModAPI.WriteDataTableValue` _modapi "GridActors" "freightDock" "toolbarGroup" _returnvalue_37)
  (`ModAPI.WriteDataTableValue` _modapi "GridActors" "freightDock" "toolbarGroupSort" "36")
  (bind _returnvalue_38 (`ModAPI.ReadDataTableValue` _modapi "GridActors" "navaltradeDock" "unlockPrerequisite"))
  (`ModAPI.WriteDataTableValue` _modapi "GridActors" "freightDock" "unlockPrerequisite" _returnvalue_38)
  (bind _returnvalue_39 (`ModAPI.ReadDataTableValue` _modapi "GridActors" "navaltradeDock" "useCustomIcon"))
  (`ModAPI.WriteDataTableValue` _modapi "GridActors" "freightDock" "useCustomIcon" _returnvalue_39)
  (bind _returnvalue_40 (`ModAPI.ReadDataTableValue` _modapi "GridActors" "navaltradeDock" "workerColor"))
  (`ModAPI.WriteDataTableValue` _modapi "GridActors" "freightDock" "workerColor" _returnvalue_40)
  (`ModAPI.AddDataTableRow` _modapi "BuildingIcons" "freightDock")
  (bind _returnvalue_41 (`ModAPI.ReadDataTableValue` _modapi "BuildingIcons" "navaltradeDock" "Icon"))
  (`ModAPI.WriteDataTableValue` _modapi "BuildingIcons" "freightDock" "Icon" _returnvalue_41)
  (`ModAPI.AddNewStrings` _modapi "dev" _map)
  (`ModAPI.AddNewStrings` _modapi "en" _map)
  (bind _returnvalue_42 (`ModAPI.ReadDataTableValue` _modapi "GridActors" "freightDock" "GridActor"))
  (bind _returnvalue_43 (`ModAPI.ReadDataTableValue` _modapi "BuildingIcons" "freightDock" "Icon"))
  (`ModAPI.LogMessage` _modapi (`KismetStringLibrary.Concat_StrStr` (`KismetStringLibrary.Concat_StrStr` (`KismetStringLibrary.Concat_StrStr` (`KismetStringLibrary.Concat_StrStr` (`KismetStringLibrary.Concat_StrStr` (`KismetStringLibrary.Concat_StrStr` (`KismetStringLibrary.Concat_StrStr` (`KismetStringLibrary.Concat_StrStr` "" "Freight dock registered: trade GridActor=") _returnvalue) ", added row ") (`KismetStringLibrary.Conv_BoolToString` _returnvalue_2)) ", GridActor=") _returnvalue_42) ", Icon=") _returnvalue_43) true))

(fn `RegisterOptions`
  (bind _modapi (`self.ModAPI`))
  (`ModAPI.RegisterModOptions` _modapi "freightdock.pairKey" "Freight Dock: pairing key" (`|MakeArray` "F1" "F2" "F3" "F4" "F5" "F6" "F7" "F8" "F9" "F10" "0") "F5" "Pairs the selected freight dock with the next one you select." :!pinned true) ; PairKey
  (`ModAPI.RegisterModOptions` _modapi "freightdock.departAfter" "Freight Dock: depart partly loaded after" (`|MakeArray` "120 s" "180 s" "240 s" "Never") "120 s" "How long a freight ship waits, from its first cargo loaded, before it sails with what it has. Never: it waits until full or nothing more is wanted." :!pinned true) ; DepartAfter
)

(fn `UserConstructionScript`)